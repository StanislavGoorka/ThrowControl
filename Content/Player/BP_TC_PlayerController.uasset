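; Player controller for a touch-based ball-throwing game, viewed through a camera tagged ThrowCamera.
; It spawns BP_Ball before the camera, respawns it when lost and prints hit scores as percentages.
; During swipes, the ball trails recent, debug-drawn touch points and rotates with curvature, summed from signed segment angles.
; On release, long enough swipes send the ball horizontal velocity from swipe speed and end position, plus curvature-based spin.
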(event `self.ReceiveBeginPlay`
  (`self.OnBeginPlay`)
  (`self.SpawnBall`))

(event `InputTouch`
  (params (Location :type "Vector Structure") (FingerIndex :type "ETouchIndex Enum"))
  (:`Pressed`
    (`self.OnTouchBegin`))
  (:`Released`
    (if (`self.bIsSwiping`)
      (set `self.bIsSwiping` false)
      (`self.OnTouchEnd`)))
  (:`Moved`
    (`self.OnTouchMove`)))

(event `/Game/Interfaces/BPI_OnBallHit.OnBallHit`
  (params (Score :type "Float (double-precision)"))
  (`KismetSystemLibrary.PrintString` (`KismetStringLibrary.Concat_StrStr` (`KismetStringLibrary.Conv_IntToString` (`KismetMathLibrary.Round` (* Score 100.0))) " %")))

(event `/Game/Interfaces/BPI_OnBallLost.OnBallLost`
  (set `self.BallREF` null)
  (`self.SpawnBall`))

(fn `CalculateSpin`
  (returns (SpinValue :type "Float (double-precision)"))
  (locals (SumAngle :type "Float (double-precision)"))
  (bind _touchpoints (`self.TouchPoints`))
  (set `local.SumAngle` 0.0)
  (for _index (range 1 (+ (- (`KismetArrayLibrary.Array_Length` _touchpoints) 2) 1))
    (bind _output (`|GetArrayItem` _touchpoints _index))
    (bind _returnvalue (`KismetMathLibrary.Normal2D` (- _output (`|GetArrayItem` _touchpoints (- _index 1)))))
    (bind _returnvalue_2 (`KismetMathLibrary.Normal2D` (- (`|GetArrayItem` _touchpoints (+ _index 1)) _output)))
    (set `local.SumAngle` (+ (`local.SumAngle`) (`KismetMathLibrary.Atan2` (`KismetMathLibrary.CrossProduct2D` _returnvalue _returnvalue_2) (`KismetMathLibrary.DotProduct2D` _returnvalue _returnvalue_2)))))
  (return (`local.SumAngle`)))

(fn `OnBeginPlay`
  (bind _throwcameraref (`self.ThrowCameraREF`))
  (bind (_x _y) (`KismetMathLibrary.BreakVector2D` (`WidgetLayoutLibrary.GetViewportSize`)))
  (`KismetSystemLibrary.ExecuteConsoleCommand` "r.ScreenPercentage 100" null)
  (`KismetSystemLibrary.ExecuteConsoleCommand` "r.MobileContentScaleFactor 1" null)
  (bind _outactors (`GameplayStatics.GetAllActorsOfClassWithTag` "/Script/Engine.CameraActor" "ThrowCamera"))
  (set `self.ThrowCameraREF` (`KismetArrayLibrary.Array_Random` _outactors))
  (`CameraComponent.SetAspectRatio` (`CameraActor.CameraComponent` (`self.ThrowCameraREF`)) (/ _x _y))
  (`CameraComponent.SetFieldOfView` (`CameraActor.CameraComponent` _throwcameraref) 45.0)
  (`self.SetViewTargetWithBlend` _throwcameraref))

(fn `OnTouchBegin`
  (bind (_locationx _locationy) (`self.GetMousePosition`))
  (bind _output_get (set `self.StartTouchPos` (`KismetMathLibrary.MakeVector2D` _locationx _locationy)))
  (set `self.CurrentTouchPos` _output_get)
  (`KismetArrayLibrary.Array_Clear` (`self.TouchPoints`))
  (`KismetArrayLibrary.Array_Add` (`self.TouchPoints`) (`self.CurrentTouchPos`))
  (set `self.TouchStartTime` (`KismetSystemLibrary.GetGameTimeInSeconds`))
  (set `self.bIsSwiping` true))

(fn `OnTouchEnd`
  (locals (SwipeTime :type "Float (double-precision)" :default 0.0) (SwipeDistance :type "Float (double-precision)" :default 0.0) (NewLocalVar :type "Float (double-precision)" :default 0.0) (SwipeVector :type "Vector2D Structure") (ThrowStrength :type "Float (double-precision)" :default 0.0) (ThrowDirection3D :type "Vector Structure" :default (0.0 0.0 0.0)) (FinalVelocity :type "Vector Structure") (SumAngle :type "Float (double-precision)"))
  (set `local.SwipeTime` (`KismetMathLibrary.FClamp` (- (`KismetSystemLibrary.GetGameTimeInSeconds`) (`self.TouchStartTime`)) 0.05))
  (bind _output_get (set `local.SwipeVector` (- (`self.CurrentTouchPos`) (`self.StartTouchPos`))))
  (bind _output_get_2 (set `local.SwipeDistance` (`KismetMathLibrary.VSize2D` _output_get)))
  (if (> _output_get_2 (`self.MinSwipeDistance`))
    (set `local.ThrowStrength` (`KismetMathLibrary.FClamp` (* (/ (`local.SwipeDistance`) (`local.SwipeTime`)) (`self.ForceMultiplier`)) 50.0 500.0))
    (set `local.ThrowDirection3D` (`KismetMathLibrary.Normal` (`KismetMathLibrary.MakeVector` (.x (`.WorldDirection` (`GameplayStatics.DeprojectScreenToWorld` self (`self.CurrentTouchPos`)))) (.y (`.WorldDirection` (`GameplayStatics.DeprojectScreenToWorld` self (`self.CurrentTouchPos`)))))))
    (set `local.FinalVelocity` (* (`local.ThrowDirection3D`) (`local.ThrowStrength`)))
    (bind _spinvalue (`self.CalculateSpin`))
    (set `self.SpinValue` (* _spinvalue (`self.SpinMultiplier`)))
    (`/Engine/EditorBlueprintResources/StandardMacros.IsValid` (`self.BallREF`)
      (:`Is Valid`
        (message `/Game/Interfaces/BPI_OnBallThrow.OnBallThrow` (`self.BallREF`) (`local.FinalVelocity`) (`self.SpinValue`)))
      (:`Is Not Valid`
        (`KismetSystemLibrary.PrintString` "No BallREF found" true true (struct :`R` 1.0 :`A` 1.0))))
    (else
      (`KismetSystemLibrary.PrintString` "Throw canceled" true true (struct :`R` 1.0 :`A` 1.0) 3.0))))

(fn `OnTouchMove`
  (bind (_locationx _locationy) (`self.GetInputTouchState` "Touch1"))
  (bind _touchpoints (`self.TouchPoints`))
  (bind _touchpoints_2 (`self.TouchPoints`))
  (bind _touchpoints_3 (`self.TouchPoints`))
  (bind _touchpoints_4 (`self.TouchPoints`))
  (bind _returnvalue (- (`KismetArrayLibrary.Array_Length` _touchpoints_2) 4))
  (bind (_worldposition _worlddirection) (`GameplayStatics.DeprojectScreenToWorld` self (`|GetArrayItem` _touchpoints_2 _returnvalue)))
  (if (`self.bIsSwiping`)
    (set `self.CurrentTouchPos` (`KismetMathLibrary.MakeVector2D` _locationx _locationy))
    (if (`KismetArrayLibrary.Array_IsValidIndex` _touchpoints_2 _returnvalue)
      (`SceneComponent.K2_SetWorldLocation` (`/Game/Game/BP_Ball.BallMesh` (`self.BallREF`)) (+ _worldposition (* _worlddirection (`self.HoldDistance`))) false false))
    (if (> (`KismetMathLibrary.Distance2D` (`self.CurrentTouchPos`) (`|GetArrayItem` _touchpoints_3 (- (`KismetArrayLibrary.Array_Length` _touchpoints_3) 1))) 3.0)
      (if (>= (`KismetArrayLibrary.Array_Length` (`self.TouchPoints`)) 30)
        (`KismetArrayLibrary.Array_Remove` (`self.TouchPoints`)))
      (`KismetArrayLibrary.Array_Add` _touchpoints_4 (`self.CurrentTouchPos`))
      (for _index (range (+ (- (`KismetArrayLibrary.Array_Length` _touchpoints_4) 2) 1))
        (bind (_worldposition_2 _worlddirection_2) (`GameplayStatics.DeprojectScreenToWorld` self (`|GetArrayItem` _touchpoints _index)))
        (bind (_worldposition_3 _worlddirection_3) (`GameplayStatics.DeprojectScreenToWorld` self (`|GetArrayItem` _touchpoints (+ _index 1))))
        (`KismetSystemLibrary.DrawDebugLine` (+ _worldposition_2 (* _worlddirection_2 100.0)) (+ _worldposition_3 (* _worlddirection_3 100.0)) (struct :`R` 1.0 :`A` 1.0) 0.0 0.5))
      (bind _spinvalue (`self.CalculateSpin`))
      (`SceneComponent.K2_AddLocalRotation` (`/Game/Game/BP_Ball.BallMesh` (`self.BallREF`)) (`KismetMathLibrary.MakeRotator` (* (`KismetMathLibrary.FClamp` _spinvalue -2.5 2.5) 10.0)) false false))))

(fn `SpawnBall`
  (bind _throwcameraref (`self.ThrowCameraREF`))
  (bind _returnvalue (`self.K2_GetActorRotation` _throwcameraref))
  (bind _returnvalue_2 (`|SpawnActorFromClass` "/Game/Game/BP_Ball.BP_Ball_C" (`KismetMathLibrary.MakeTransform` (+ (`self.K2_GetActorLocation` _throwcameraref) (* (`self.HoldDistance`) (`KismetMathLibrary.GetForwardVector` _returnvalue))) _returnvalue) "Undefined" "MultiplyWithRoot" null null))
  (bind _output_get (set `self.BallREF` _returnvalue_2))
  (`PrimitiveComponent.SetSimulatePhysics` (`/Game/Game/BP_Ball.BallMesh` _output_get) false))

(fn `UserConstructionScript`)