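; BP_Ball is a throwable physics ball that curves sideways in flight according to its spin.
; OnBallThrow stores the spin, enables physics on BallMesh, then applies the velocity as an impulse and a spin-scaled torque around the mesh's right vector.
; Once thrown, Tick fakes a Magnus-like curve with a horizontal acceleration perpendicular to velocity, scaled by spin and CurveStrength but independent of speed.
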(event `/Game/Interfaces/BPI_OnBallThrow.OnBallThrow`
  (params (Velocity :type "Vector Structure") (Spin :type "Float (double-precision)"))
  (bind _ballmesh (`self.BallMesh`))
  (set `self.SpinValue` Spin)
  (`PrimitiveComponent.SetSimulatePhysics` _ballmesh true)
  (`PrimitiveComponent.AddImpulse` _ballmesh Velocity "None" true)
  (`PrimitiveComponent.AddTorqueInRadians` _ballmesh (* (`SceneComponent.GetRightVector` _ballmesh) (`self.SpinValue`) 500.0) "None" false)
  (set `self.bIsThrown` true))

(event `self.ReceiveTick`
  (params (DeltaSeconds :type "Float (single-precision)"))
  (if (`self.bIsThrown`)
    (bind _returnvalue (`PrimitiveComponent.GetPhysicsLinearVelocity` (`self.BallMesh`) "None"))
    (`PrimitiveComponent.AddForce` (`self.BallMesh`) (* (`KismetMathLibrary.Normal` (`KismetMathLibrary.Cross_VectorVector` _returnvalue (`KismetMathLibrary.MakeVector` 0.0 0.0 1.0))) (`self.SpinValue`) (`self.CurveStrength`)) "None" true)))

(fn `UserConstructionScript`)