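; BP_Target is a target actor that reports how close to its center a hit lands.
; On BeginPlay it fits TriggerBox around the Cylinder's bounds with some padding and binds its begin overlap.
; Any overlap sends the player controller a score from 1 at center to 0 at the edge, using YZ-plane distance normalized by the Cylinder's bounds radius.
; The actor-hit binding and BP_Ball check are unconnected leftovers.
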(event `self.ReceiveBeginPlay`
  (bind _triggerbox (`self.TriggerBox`))
  (bind (_origin _boxextent) (`KismetSystemLibrary.GetComponentBounds` (`self.Cylinder`)))
  (`BoxComponent.SetBoxExtent` _triggerbox (* _boxextent 1.3) true)
  (`SceneComponent.K2_SetWorldLocation` _triggerbox _origin false false)
  (add `PrimitiveComponent.OnComponentBeginOverlap` (`self.TriggerBox`) (delegate `OnTriggerBoxBeginOverlap`)))

(event `OnTriggerBoxBeginOverlap`
  (params (OverlappedComponent :type "PrimitiveComponent Object Reference") (OtherActor :type "Actor Object Reference") (OtherComp :type "PrimitiveComponent Object Reference") (OtherBodyIndex :type Integer) (bFromSweep :type Boolean) (SweepResult :type "HitResult Structure (by ref)"))
  (message `/Game/Interfaces/BPI_OnBallHit.OnBallHit` (`GameplayStatics.GetPlayerController` 0) (`KismetMathLibrary.Abs` (- (`KismetMathLibrary.FClamp` (/ (`KismetMathLibrary.Distance2D` (`KismetMathLibrary.MakeVector2D` (.y (`SceneComponent.K2_GetComponentLocation` OtherComp)) (.z (`SceneComponent.K2_GetComponentLocation` OtherComp))) (`KismetMathLibrary.MakeVector2D` (.y (`self.K2_GetActorLocation`)) (.z (`self.K2_GetActorLocation`)))) (`.SphereRadius` (`KismetSystemLibrary.GetComponentBounds` (`self.Cylinder`))))) 1.0))))

(event `OnActorHit_Event` :!signature `self.OnActorHit`
  (params (SelfActor :type "Actor Object Reference") (OtherActor :type "Actor Object Reference") (NormalImpulse :type "Vector Structure") (Hit :type "HitResult Structure (by ref)")))

(fn `UserConstructionScript`)